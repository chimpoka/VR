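; BP_Button is a VR interactable that the player fills up through repeated grabs.
; Motion controllers overlapping its sphere bind that hand's grab event on the MotionControllerPawn, and unbind it on leaving.
; Each grab increments a widget progress bar, while Tick drains it over time.
; Reaching full fires the OnProgressFull dispatcher and latches the button, stopping further changes.
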(event `self.ReceiveBeginPlay`
  (bind _aswbp_progress_bar (cast `/Game/Blueprints/Button/WBP_ProgressBar` (`WidgetComponent.GetUserWidgetObject` (`self.Widget`))))
  (set `self.ProgressBar` _aswbp_progress_bar)
  (bind _asmotion_controller_pawn (cast `/Game/VirtualRealityBP/Blueprints/MotionControllerPawn` (`GameplayStatics.GetPlayerPawn` 0)))
  (set `self.Player` _asmotion_controller_pawn))

(event `self.OverlapSphere.OnComponentBeginOverlap`
  (params (OverlappedComponent :type "PrimitiveComponent Object Reference") (OtherActor :type "Actor Object Reference") (OtherComp :type "PrimitiveComponent Object Reference") (OtherBodyIndex :type Integer) (bFromSweep :type Boolean) (SweepResult :type "HitResult Structure (by ref)"))
  (bind _player (`self.Player`))
  (bind _asbp_motion_controller (cast `/Game/VirtualRealityBP/Blueprints/BP_MotionController` OtherActor))
  (switch `EControllerHand` (`/Game/VirtualRealityBP/Blueprints/BP_MotionController.Hand` _asbp_motion_controller)
    (:`Left`
      (add `/Game/VirtualRealityBP/Blueprints/MotionControllerPawn.OnGrabLeft` _player (delegate `OnGrab_Event`)))
    (:`Right`
      (add `/Game/VirtualRealityBP/Blueprints/MotionControllerPawn.OnGrabRight` _player (delegate `OnGrab_Event`)))))

(event `self.OverlapSphere.OnComponentEndOverlap`
  (params (OverlappedComponent :type "PrimitiveComponent Object Reference") (OtherActor :type "Actor Object Reference") (OtherComp :type "PrimitiveComponent Object Reference") (OtherBodyIndex :type Integer))
  (bind _asbp_motion_controller (cast `/Game/VirtualRealityBP/Blueprints/BP_MotionController` OtherActor))
  (switch `EControllerHand` (`/Game/VirtualRealityBP/Blueprints/BP_MotionController.Hand` _asbp_motion_controller)
    (:`Left`
      (remove `/Game/VirtualRealityBP/Blueprints/MotionControllerPawn.OnGrabLeft` (`self.Player`) (delegate `OnGrab_Event`)))
    (:`Right`
      (remove `/Game/VirtualRealityBP/Blueprints/MotionControllerPawn.OnGrabRight` (`self.Player`) (delegate `OnGrab_Event`)))))

(event `OnGrab_Event`
  (if (not (`self.bProgressFull`))
    ;[0 0 0] Increasing progerss bar
    (bind _output_get (set `self.Progress` (+ (`self.IncrementSpeed`) (`self.Progress`))))
    (`/Game/Blueprints/Button/WBP_ProgressBar.SetProgress` (`self.ProgressBar`) _output_get)
    (if (>= (`self.Progress`) 1.0)
      (`self.OnProgressFull_Event`))))

(event `self.ReceiveTick`
  (params (DeltaSeconds :type "Float (single-precision)"))
  (set `self.DeltaT` DeltaSeconds)
  (if (> (`self.Progress`) 0.0)
    (if (not (`self.bProgressFull`))
      ;[0 0 0] Decreasing Progress Bar
      (bind _output_get (set `self.Progress` (- (`self.Progress`) (* (`self.DeltaT`) (`self.DecrementSpeed`)))))
      (`/Game/Blueprints/Button/WBP_ProgressBar.SetProgress` (`self.ProgressBar`) _output_get))))

(event `OnProgressFull_Event`
  (`self.OnProgressFull`)
  (set `self.bProgressFull` true))

(fn `UserConstructionScript`)