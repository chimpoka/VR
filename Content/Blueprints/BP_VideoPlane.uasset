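; BP_VideoPlane is an actor that rises into view and then opens a video.
; ShowUp sets a Showing flag, which makes Tick move the actor along local Z at ShowUpSpeed until the accumulated offset reaches ShowUpHeight.
; The show-up event then fires the OnShowUp dispatcher, stops the movement and calls ShowVideo to open the MediaSource on the MediaPlayer.
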(event `self.ReceiveTick`
  (params (DeltaSeconds :type "Float (single-precision)"))
  (bind _returnvalue (* (`self.ShowUpSpeed`) (`self.DeltaT`)))
  (set `self.DeltaT` DeltaSeconds)
  (if (`self.bShowing`)
    ;[0 0 0] Increasing plane Z position
    (set `self.CurrentShowUpHeight` (+ (`self.CurrentShowUpHeight`) _returnvalue))
    (`self.K2_AddActorLocalOffset` (`KismetMathLibrary.MakeVector` 0.0 0.0 _returnvalue))
    (if (>= (`self.CurrentShowUpHeight`) (`self.ShowUpHeight`))
      (`self.OnShowUp_Event`))))

(event `OnShowUp_Event`
  (`self.OnShowUp`)
  (set `self.bShowing` false)
  (`self.ShowVideo`))

(fn `ShowUp`
  (set `self.bShowing` true))

(fn `ShowVideo`
  (`MediaPlayer.OpenSource` (`self.MediaPlayer`) (`self.MediaSource`)))

(fn `UserConstructionScript`)